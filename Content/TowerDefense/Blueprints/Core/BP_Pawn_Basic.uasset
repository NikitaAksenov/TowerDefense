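; BP_Pawn_Basic is a basic pawn in the TowerDefense project that the player moves with Enhanced Input actions.
; IA_MoveForward and IA_MoveRight scale the actor's forward and right vectors by their action values and pass the result to a shared Move function.
; Move applies a world offset scaled by MoveSpeed and frame delta time, without sweeping, so movement performs no collision check.
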(event `EnhancedInput|/Game/TowerDefense/Blueprints/Input/Actions/IA_MoveForward`
  (params (ActionValue :type "Float (double-precision)") (ElapsedSeconds :type "Float (double-precision)") (TriggeredSeconds :type "Float (double-precision)") (InputAction :type "InputAction Object Reference" :default "/Game/TowerDefense/Blueprints/Input/Actions/IA_MoveForward.IA_MoveForward"))
  (:`Triggered`
    (`self.Move` (* (`self.GetActorForwardVector`) ActionValue))))

(event `EnhancedInput|/Game/TowerDefense/Blueprints/Input/Actions/IA_MoveRight`
  (params (ActionValue :type "Float (double-precision)") (ElapsedSeconds :type "Float (double-precision)") (TriggeredSeconds :type "Float (double-precision)") (InputAction :type "InputAction Object Reference" :default "/Game/TowerDefense/Blueprints/Input/Actions/IA_MoveRight.IA_MoveRight"))
  (:`Triggered`
    (`self.Move` (* (`self.GetActorRightVector`) ActionValue))))

(fn `Move`
  (params (MoveVector :type "Vector Structure"))
  (`self.K2_AddActorWorldOffset` (* MoveVector (`GameplayStatics.GetWorldDeltaSeconds`) (`self.MoveSpeed`))))

(fn `UserConstructionScript`)